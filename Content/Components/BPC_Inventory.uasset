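; Player inventory component that holds items as class and amount slots, sized from BP_CryptController, and links an examination widget.
; AddItem recursively spreads amounts across slots by max stack, but CheckForFreeSlot always returns failure, so existing stacks never merge.
; UseItem calls UseItem on a found or spawned item actor, then decrements the slot.
; DropItem empties a slot and spawns a physics pickup at a camera trace; UpdateInventorySlot is an empty stub.
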(event Custom|Initialize
  (bind _returnvalue (Game|GetPlayerController 0))
  (bind _asbp_crypt_controller (Utilities|Casting|CastToBP_CryptController _returnvalue))
  (Utilities|Array|Resize (Variables|Default|GetInventorySlots) (Variables|/Game/Actors/Controller/BP_CryptController.BP_CryptController_C|GetInventorySlot _asbp_crypt_controller))
  (Variables|Default|SetUI%20Inventory%20Menu (Variables|/Game/Actors/Controller/BP_CryptController.BP_CryptController_C|GetUI%20Inventory%20Menu _asbp_crypt_controller))
  (bind _asbp_player (Utilities|Casting|CastToBP_Player (Game|GetPlayerCharacter 0)))
  (Variables|Default|SetPlayerRef _asbp_player)
  (bind _returnvalue_2 (Game|ConstructObjectfromClass "/Game/UI/Inventory/UI_Examination.UI_Examination_C" 0))
  (Variables|Default|SetUI_ExaminationRef _returnvalue_2)
  (bind _outactors (Actor|GetAllActorsOfClass "/Game/Actors/Inventory/BP_Examination.BP_Examination_C"))
  (Variables|Default|SetBP_Examination (Utilities|Array|Get(acopy) _outactors))
  (Variables|/Game/UI/Inventory/UI_Examination.UI_Examination_C|SetBPC_InventoryRef (Variables|Default|GetUI_ExaminationRef) self))

(event Custom|CreateExaminationWidget
  (params (Index :type Integer))
  (Default|UpdateWidget (Variables|Default|GetUI_ExaminationRef) Index))

(event EventBeginPlay
  (CallFunction|Initialize))

(fn AddItem
  (params (Item :type BP%20Inventory%20Item%20Master%20Class%20Reference) (Amount :type Integer))
  (bind (_success _outindex) (CallFunction|CheckforEmptySlot))
  (bind (_success_2 _outindex_2) (CallFunction|CheckforEmptySlot))
  ;[1 1 1] Local Item(Inventory) 개수와 남은 자리 현재 습득하는 아이템 정보 얻기
  (LocalVariables|SetLocalItem Item)
  (LocalVariables|SetLocalAmount Amount)
  (LocalVariables|SetLocalMaxStackAmount (.MaxStackAmount (Utilities|Struct|BreakS_ItemData (Utilities|GetClassDefaults (LocalVariables|GetLocalItem)))))
  (if (> (.MaxStackAmount (Utilities|Struct|BreakS_ItemData (Utilities|GetClassDefaults (LocalVariables|GetLocalItem)))) 1)
    (bind (_sucess_ _index) (CallFunction|CheckforFreeSlot (LocalVariables|GetLocalItem)))
    (if _sucess_
      (LocalVariables|SetLocalIndex _index)
      (if (> (+ (.Amount (CallFunction|GetItemDataIndex (LocalVariables|GetLocalIndex))) (LocalVariables|GetLocalAmount)) (LocalVariables|GetLocalMaxStackAmount))
        (LocalVariables|SetLocalAmount (- (+ (.Amount (CallFunction|GetItemDataIndex (LocalVariables|GetLocalIndex))) (LocalVariables|GetLocalAmount)) (LocalVariables|GetLocalMaxStackAmount)))
        (Utilities|Array|SetArrayElem (Variables|Default|GetInventorySlots) (LocalVariables|GetLocalIndex) (Utilities|Struct|MakeS_InventoryItem (LocalVariables|GetLocalItem) (LocalVariables|GetLocalMaxStackAmount)))
        (CallFunction|UpdateInventorySlot (LocalVariables|GetLocalIndex))
        (bind _remainder (CallFunction|AddItem (LocalVariables|GetLocalItem) (LocalVariables|GetLocalAmount)))
        (return true _remainder)
        (else
          (Utilities|Array|SetArrayElem (Variables|Default|GetInventorySlots) (LocalVariables|GetLocalIndex) (Utilities|Struct|MakeS_InventoryItem (LocalVariables|GetLocalItem) (+ (.Amount (CallFunction|GetItemDataIndex (LocalVariables|GetLocalIndex))) (LocalVariables|GetLocalAmount))))
          (CallFunction|UpdateInventorySlot (LocalVariables|GetLocalIndex))
          (return true 0)))
      (elif _success_2
        (LocalVariables|SetLocalIndex _outindex_2)
        (if (> (LocalVariables|GetLocalAmount) (LocalVariables|GetLocalMaxStackAmount))
          (Utilities|Array|SetArrayElem (Variables|Default|GetInventorySlots) (LocalVariables|GetLocalIndex) (Utilities|Struct|MakeS_InventoryItem (LocalVariables|GetLocalItem) (LocalVariables|GetLocalMaxStackAmount)))
          (CallFunction|UpdateInventorySlot (LocalVariables|GetLocalIndex))
          (CallFunction|AddItem (LocalVariables|GetLocalItem) (- (LocalVariables|GetLocalAmount) (LocalVariables|GetLocalMaxStackAmount)))
          (else
            (Utilities|Array|SetArrayElem (Variables|Default|GetInventorySlots) (LocalVariables|GetLocalIndex) (Utilities|Struct|MakeS_InventoryItem (LocalVariables|GetLocalItem) (LocalVariables|GetLocalAmount)))
            (CallFunction|UpdateInventorySlot (LocalVariables|GetLocalIndex))
            (return true 0)))
        (else
          (return false (LocalVariables|GetLocalAmount)))))
    (else
      ;[1 1 1] 빈자리 체크해서 실패출력
      (if _success
        (LocalVariables|SetLocalIndex _outindex)
        (Utilities|Array|SetArrayElem (Variables|Default|GetInventorySlots) (LocalVariables|GetLocalIndex) (Utilities|Struct|MakeS_InventoryItem (LocalVariables|GetLocalItem) 1))
        (CallFunction|UpdateInventorySlot (LocalVariables|GetLocalIndex))
        (if (> (- (LocalVariables|GetLocalAmount) 1) 0)
          (bind _remainder_2 (CallFunction|AddItem (LocalVariables|GetLocalItem) (- (LocalVariables|GetLocalAmount) 1)))
          (return true _remainder_2)
          (else
            (return true 0)))
        (else
          (Development|PrintString "NoFreeSlot")
          (return false 0))))))

(fn CheckforEmptySlot
  (bind (_array_element _array_index) (Utilities|Array|ForEachLoopwithBreak (Variables|Default|GetInventorySlots) :!label _label)
    (:LoopBody
      (if (Utilities|IsValidClass (.Item (Utilities|Struct|BreakS_InventoryItem _array_element)))
        (LocalVariables|SetLocalSuccess false)
        (else
          (LocalVariables|SetLocalSuccess true)
          (LocalVariables|SetLocalIndex _array_index)
          (goto _label Break))))
    (:Completed
      (return (LocalVariables|GetLocalSuccess) (LocalVariables|GetLocalIndex)))))

(fn GetItemDataIndex
  (params (Index :type Integer))
  (bind _inventoryslots (Variables|Default|GetInventorySlots))
  (bind _output (Utilities|Array|Get(acopy) _inventoryslots Index))
  (bind (_item _amount) (Utilities|Struct|BreakS_InventoryItem _output))
  ;[1 1 1] 완료
  (return _item _amount))

(fn UpdateInventorySlot
  (params (Index :type Integer)))

(fn CheckforFreeSlot
  (params (Item :type BP%20Inventory%20Item%20Master%20Class%20Reference))
  (bind (_array_element _array_index) (Utilities|Array|ForEachLoopwithBreak (Variables|Default|GetInventorySlots) :!label _label)
    (:LoopBody
      (if (and (== (.Item (Utilities|Struct|BreakS_InventoryItem _array_element)) Item) (< (.Amount (Utilities|Struct|BreakS_InventoryItem _array_element)) (.maxstackamount (Utilities|GetClassDefaults Item))))
        (LocalVariables|SetLocalSucess true)
        (LocalVariables|SetLocalIndex _array_index)
        (goto _label Break)
        (else
          (LocalVariables|SetLocalSucess true))))
    (:Completed
      (return false (LocalVariables|GetLocalIndex)))))

(fn UseItem
  (params (Index :type Integer))
  (bind _output_get (LocalVariables|SetLocalIndex Index))
  (bind _returnvalue (Actor|GetActorOfClass (.Item (CallFunction|GetItemDataIndex _output_get))))
  (Utilities|IsValid _returnvalue
    (:Is%20Valid
      (Default|UseItem _returnvalue))
    (:Is%20Not%20Valid
      (bind _returnvalue_2 (Game|SpawnActorfromClass (.Item (CallFunction|GetItemDataIndex _output_get)) (Math|Transform|MakeTransform "0, 0, 0" "0, 0, 0" "1.000000,1.000000,1.000000") "Undefined" "MultiplyWithRoot" 0 0))
      (Default|UseItem _returnvalue_2)))
  (CallFunction|RemoveItem (LocalVariables|GetLocalIndex)))

(fn RemoveItem
  (params (NewParam :type Integer))
  (bind (_item _amount) (CallFunction|GetItemDataIndex NewParam))
  (if (> _amount 1)
    (Utilities|Array|SetArrayElem (Variables|Default|GetInventorySlots) NewParam (Utilities|Struct|MakeS_InventoryItem _item (- _amount 1)))
    (else
      (Utilities|Array|SetArrayElem (Variables|Default|GetInventorySlots) NewParam (Utilities|Struct|MakeS_InventoryItem 0 0))))
  (CallFunction|UpdateInventorySlot NewParam))

(fn DropItem
  (params (Index :type Integer))
  (bind _playerref (Variables|Default|GetPlayerRef))
  (bind _firstpersoncameracomponent (Variables|/Script/CryptRider.CryptRiderCharacter|GetFirstPersonCameraComponent _playerref))
  (bind _returnvalue (Transformation|GetWorldLocation _firstpersoncameracomponent))
  (bind _output_get (LocalVariables|SetLocalIndex Index))
  (LocalVariables|SetLocalAmount (.Amount (CallFunction|GetItemDataIndex _output_get)))
  (LocalVariables|SetLocalClass (.Item (CallFunction|GetItemDataIndex _output_get)))
  (if (> (LocalVariables|GetLocalAmount) 0)
    (for _index (range 0 (- (LocalVariables|GetLocalAmount) 1))
      (CallFunction|RemoveItem (LocalVariables|GetLocalIndex)))
    (bind (_outhit _returnvalue_2) (Collision|LineTraceByChannel _returnvalue (+ _returnvalue (* (Math|Vector|GetForwardVector _firstpersoncameracomponent) 2e+02)) "TraceTypeQuery1" false 0 "None"))
    (bind _returnvalue_3 (Game|SpawnActorfromClass (.BPickUp (Utilities|Struct|BreakS_ItemData (Utilities|GetClassDefaults (LocalVariables|GetLocalClass)))) (select _returnvalue_2 (Math|Conversions|ToTransform(Vector) (.Location (Collision|BreakHitResult _outhit))) (Math|Conversions|ToTransform(Vector) (.TraceEnd (Collision|BreakHitResult _outhit)))) "Undefined" "MultiplyWithRoot" 0 0))
    (Variables|/Game/Actors/Inventory/PickUpActors/BP_PickupActor_Master.BP_PickupActor_Master_C|SetAmount _returnvalue_3 (LocalVariables|GetLocalAmount))
    (Physics|SetSimulatePhysics (Variables|/Game/Actors/Inventory/PickUpActors/BP_PickupActor_Master.BP_PickupActor_Master_C|GetStaticMesh _returnvalue_3) true)))