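; BP_Player is the player Blueprint, with input hooks for inventory and return actions, though its live logic is mostly stubbed.
; IA_InventoryToggle calls an empty ToggleInventory event, and IA_Return binds a touch-begin delegate to an empty handler.
; Disconnected nodes hold a pause toggle for movement, cursor, input mode and visibility, plus UI widget creation, none of which runs.
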(event Custom|ToggleInventory)

(event Custom|OnInputTouchBegin_Event
  (params (FingerIndex :type ETouchIndex%20Enum :default "Touch1") (TouchedActor :type Actor%20Object%20Reference)))

(event Input|EnhancedActionEvents|EnhancedInputActionIA_InventoryToggle
  (params (ActionValue :type Boolean) (ElapsedSeconds :type Float%20%28double-precision%29) (TriggeredSeconds :type Float%20%28double-precision%29) (InputAction :type Input%20Action%20Object%20Reference :default "/Game/Input/IA_InventoryToggle.IA_InventoryToggle"))
  (CallFunction|ToggleInventory))

(event Input|EnhancedActionEvents|EnhancedInputActionIA_Return
  (params (ActionValue :type Boolean) (ElapsedSeconds :type Float%20%28double-precision%29) (TriggeredSeconds :type Float%20%28double-precision%29) (InputAction :type Input%20Action%20Object%20Reference :default "/Game/Input/IA_Return.IA_Return"))
  (EventDispatchers|BindEventtoOnInputTouchBegin (delegate Custom|OnInputTouchBegin_Event)))

(event EventBeginPlay
  (|CallParentFunction))

(fn ConstructionScript
  (|CallParentFunction))