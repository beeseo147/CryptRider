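; A single dial of a combination lock that turns in 36-degree steps, one per number.
; Up and down arrow widgets receive a reference to the dial and their direction at BeginPlay.
; One timeline, played forward or reversed, animates the mesh roll, then updates the stored angle, derives Number and has the lock run CheckEveryTurn.
; A Rotation flag gates input, but only backward turns clear it while animating.
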(event Custom|FindNumber
  (bind _output_get (Variables|Default|SetNumber (Math|Float|Truncate (/ (Class|KismetMathLibrary|ClampAxis (.roll (Variables|/Script/Engine.SceneComponent|GetRelativeRotation (Variables|Default|GetDialMesh)))) 36.0))))
  (Development|PrintString (Utilities|String|ToString(Integer) _output_get)))

(event Custom|RotationDiar
  (if (Variables|Default|GetbRotation)
    (Variables|Default|SetbRotation true)
    (bind (_direction _새_트랙_0) (Timeline|DiarRotationTL PlayFromStart)
      (:Update
        (Transformation|SetRelativeRotation (Variables|Default|GetDialMesh) (Math|Rotator|MakeRotator (+ (Utilities|Select :Index _direction :Forward (Math|Float|Lerp 0.0 36.0 _새_트랙_0) :Backward (Math|Float|Lerp -36.0 0.0 _새_트랙_0)) (Variables|Default|GetDiarRotation)) 0.0 0.0) false false))
      (:Finished
        (Variables|Default|SetDiarRotation (+ (Utilities|Select :Index _direction :Forward (Math|Float|Lerp 0.0 36.0 _새_트랙_0) :Backward (Math|Float|Lerp -36.0 0.0 _새_트랙_0)) (Variables|Default|GetDiarRotation)))
        (if (>= (Class|KismetMathLibrary|ClampAxis (Variables|Default|GetDiarRotation)) 3.6e+02)
          (Variables|Default|SetDiarRotation 0.0)
          (Transformation|SetRelativeRotation (Variables|Default|GetDialMesh) "0, 0, 0" false false)
          (elif (< (Class|KismetMathLibrary|ClampAxis (Variables|Default|GetDiarRotation)) 0.0)
            (bind _output_get (Variables|Default|SetDiarRotation (Math|Float|MapRangeClamped (Variables|Default|GetDiarRotation) 0.0 -3.6e+02 3.6e+02 0.0)))
            (Transformation|SetRelativeRotation (Variables|Default|GetDialMesh) (Math|Rotator|MakeRotator _output_get 0.0 0.0) false false)))
        (CallFunction|FindNumber)
        (Default|CheckEveryTurn (Variables|Default|GetBPLockRef))
        (Variables|Default|SetbRotation true)))))

(event Custom|RotateDiarBackward
  (if (Variables|Default|GetbRotation)
    (Variables|Default|SetbRotation false)
    (bind (_direction _새_트랙_0) (Timeline|DiarRotationTL ReverseFromEnd)
      (:Update
        (Transformation|SetRelativeRotation (Variables|Default|GetDialMesh) (Math|Rotator|MakeRotator (+ (Utilities|Select :Index _direction :Forward (Math|Float|Lerp 0.0 36.0 _새_트랙_0) :Backward (Math|Float|Lerp -36.0 0.0 _새_트랙_0)) (Variables|Default|GetDiarRotation)) 0.0 0.0) false false))
      (:Finished
        (Variables|Default|SetDiarRotation (+ (Utilities|Select :Index _direction :Forward (Math|Float|Lerp 0.0 36.0 _새_트랙_0) :Backward (Math|Float|Lerp -36.0 0.0 _새_트랙_0)) (Variables|Default|GetDiarRotation)))
        (if (>= (Class|KismetMathLibrary|ClampAxis (Variables|Default|GetDiarRotation)) 3.6e+02)
          (Variables|Default|SetDiarRotation 0.0)
          (Transformation|SetRelativeRotation (Variables|Default|GetDialMesh) "0, 0, 0" false false)
          (elif (< (Class|KismetMathLibrary|ClampAxis (Variables|Default|GetDiarRotation)) 0.0)
            (bind _output_get (Variables|Default|SetDiarRotation (Math|Float|MapRangeClamped (Variables|Default|GetDiarRotation) 0.0 -3.6e+02 3.6e+02 0.0)))
            (Transformation|SetRelativeRotation (Variables|Default|GetDialMesh) (Math|Rotator|MakeRotator _output_get 0.0 0.0) false false)))
        (CallFunction|FindNumber)
        (Default|CheckEveryTurn (Variables|Default|GetBPLockRef))
        (Variables|Default|SetbRotation true)))))

(event EventBeginPlay
  (Default|Initialize (.AsUI%20Arrow (Utilities|Casting|CastToUI_Arrow (UserInterface|GetUserWidgetObject (Variables|Default|GetUpArrow)))) self true)
  (Default|Initialize (.AsUI%20Arrow (Utilities|Casting|CastToUI_Arrow (UserInterface|GetUserWidgetObject (Variables|Default|GetDownArrow)))) self false))

(event EventTick
  (params (DeltaSeconds :type Float%20%28single-precision%29)))

(fn ConstructionScript)