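; BP_NoteMater is a note actor that shows a floating pickup prompt to the Crypt Rider player and writes its text in construction.
; Sphere overlap starts and stops per-tick updates.
; While active, a visibility trace to the player's camera hides the prompt if blocked, otherwise turns it toward the camera.
; Trace length against the pickup distance toggles the prompt state and actor input; no input handler is defined here.
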(event OnComponentEndOverlap(Sphere)
  (params (OverlappedComponent :type Primitive%20Component%20Object%20Reference) (OtherActor :type Actor%20Object%20Reference) (OtherComp :type Primitive%20Component%20Object%20Reference) (OtherBodyIndex :type Integer))
  (bind _prompt (Variables|Default|GetPrompt))
  (Utilities|IsValid self
    (:Is%20Valid
      (Utilities|IsValid _prompt
        (:Is%20Valid
          (Rendering|SetVisibility _prompt false false)
          (Variables|Default|SetUpdateActor false)
          (Input|DisableInput (Game|GetPlayerController 0)))))))

(event OnComponentBeginOverlap(Sphere)
  (params (OverlappedComponent :type Primitive%20Component%20Object%20Reference) (OtherActor :type Actor%20Object%20Reference) (OtherComp :type Primitive%20Component%20Object%20Reference) (OtherBodyIndex :type Integer) (bFromSweep :type Boolean) (SweepResult :type Hit%20Result%20Structure%20%28by%20ref%29))
  (bind _asbp_crypt_rider_character (Utilities|Casting|CastToBP_CryptRiderCharacter OtherActor))
  (Variables|Default|SetPlayer _asbp_crypt_rider_character)
  (Rendering|SetVisibility (Variables|Default|GetPrompt) true false)
  (Variables|Default|SetUpdateActor true))

(event EventTick
  (params (DeltaSeconds :type Float%20%28single-precision%29))
  (bind _returnvalue (Game|GetPlayerController 0))
  (bind _paper (Variables|Default|GetPaper))
  (bind _prompt (Variables|Default|GetPrompt))
  (bind _returnvalue_2 (Transformation|GetWorldLocation _paper))
  (Transformation|SetWorldLocation (Variables|Default|GetPrompt) (Math|Vector|MakeVector (.x _returnvalue_2) (.y _returnvalue_2) (+ (.z _returnvalue_2) (Variables|Default|GetWidgetDistanceAboutMesh))) false false)
  (if (Variables|Default|GetUpdateActor)
    (bind (_outhit _returnvalue_3) (Collision|LineTraceByChannel (Transformation|GetActorLocation) (Transformation|GetWorldLocation (Variables|/Script/CryptRider.CryptRiderCharacter|GetFirstPersonCameraComponent (Variables|Default|GetPlayer))) "TraceTypeQuery1" false 0 "None"))
    (if (not _returnvalue_3)
      (Rendering|SetVisibility _prompt true false)
      (Transformation|SetWorldRotation (Variables|Default|GetPrompt) (Math|Rotator|FindLookatRotation (Transformation|GetWorldLocation (Variables|Default|GetPrompt)) (Transformation|GetWorldLocation (Variables|/Script/CryptRider.CryptRiderCharacter|GetFirstPersonCameraComponent (Variables|Default|GetPlayer)))) false false)
      (Default|TogglePrompt (.AsUI%20Pick%20Up%20Prompt (Utilities|Casting|CastToUI_PickUpPrompt (UserInterface|GetUserWidgetObject (Variables|Default|GetPrompt)))) (<= (Math|Vector|VectorLength (- (.TraceStart (Collision|BreakHitResult _outhit)) (.TraceEnd (Collision|BreakHitResult _outhit)))) (Variables|Default|GetPickUpDistance)))
      (if (<= (Math|Vector|VectorLength (- (.TraceStart (Collision|BreakHitResult _outhit)) (.TraceEnd (Collision|BreakHitResult _outhit)))) (Variables|Default|GetPickUpDistance))
        (Input|EnableInput _returnvalue)
        (else
          (Input|DisableInput _returnvalue)))
      (else
        (Rendering|SetVisibility _prompt false false)
        (Input|DisableInput (Game|GetPlayerController 0))))))

(event Collision|EventActorBeginOverlap
  (params (OtherActor :type Actor%20Object%20Reference)))

(event EventBeginPlay)

(fn ConstructionScript
  (Rendering|Components|TextRender|SetText (Variables|Default|GetNoteText) (Variables|Default|GetValue)))